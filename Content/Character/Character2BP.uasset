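; Character2BP is a character Blueprint with custom movement and weapon holder components, largely inherited setup plus debug scaffolding.
; BeginPlay calls the parent, then applies a stored property set to the CharacterMovement2 component.
; Pressing 1 writes every actor's display name to the log without showing it on screen.
; Disconnected, never-executed experiments cover render-target drawing, garbage collection, automatic weapon fire for non-local characters and AI turn-toward-movement rotation.
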(event EventBeginPlay
  (|CallParentFunction)
  (Class|CharacterMovementComponent2|SetCharacterMovementProperties (Variables|Default|GetCharacterMovement2) (Variables|Default|GetNewVar_2)))

(event Input|KeyboardEvents|1
  (params (Key :type Key%20Structure :default "None"))
  (:Pressed
    (bind _outactors (Actor|GetAllActorsOfClass "/Script/Engine.Actor"))
    (for _array_element _outactors
      (Development|PrintString (Utilities|GetDisplayName _array_element) false true "(R=0.000000,G=0.660000,B=1.000000,A=1.000000)" 1e+01))))

(fn ConstructionScript)